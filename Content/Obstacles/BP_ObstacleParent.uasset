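; BP_ObstacleParent is a base obstacle that temporarily disappears when hit by a projectile of matching light/dark value.
; On a static mesh hit, it compares the BP_ProjectileParent's ProjectileValue to its own LightDarkValue.
; A match toggles visibility and disables collision, then reverses both after a fixed delay.
; BeginPlay calls SetCharacterTagValue, which is empty in this class.
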(event `self.ReceiveBeginPlay`
  (`self.SetCharacterTagValue`))

(event `self.StaticMesh.OnComponentHit`
  (params (HitComponent :type "PrimitiveComponent Object Reference") (OtherActor :type "Actor Object Reference") (OtherComp :type "PrimitiveComponent Object Reference") (NormalImpulse :type "Vector Structure") (Hit :type "HitResult Structure (by ref)"))
  ;[1 1 1] Toggle Collision and Visibility of Hit object
  (bind _asbp_projectile_parent (cast `/Game/Projectiles/Blueprints/BP_ProjectileParent` OtherActor))
  (if (== (`/Game/Projectiles/Blueprints/BP_ProjectileParent.ProjectileValue` _asbp_projectile_parent) (`self.LightDarkValue`))
    (`SceneComponent.ToggleVisibility` (`self.StaticMesh`) false)
    (`PrimitiveComponent.SetCollisionEnabled` (`self.StaticMesh`) "NoCollision")
    (`KismetSystemLibrary.Delay` 5.0)
    (`SceneComponent.ToggleVisibility` (`self.StaticMesh`) false)
    (`PrimitiveComponent.SetCollisionEnabled` (`self.StaticMesh`) "QueryAndPhysics")))

(fn `SetCharacterTagValue`)

(fn `UserConstructionScript`)