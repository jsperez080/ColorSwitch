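; Parent Blueprint for a color puzzle piece that toggles between Light and Dark when hit by a projectile of matching value.
; A matching hit raises IsHit, swaps material and state, then clears the flag after a brief delay so a processor can react.
; ChangeAdjacentPuzzlePiece swaps a target piece's material by the target's state, but writes the new value to its own LightDarkValue.
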(event `self.StaticMesh.OnComponentHit`
  (params (HitComponent :type "PrimitiveComponent Object Reference") (OtherActor :type "Actor Object Reference") (OtherComp :type "PrimitiveComponent Object Reference") (NormalImpulse :type "Vector Structure") (Hit :type "HitResult Structure (by ref)"))
  ;[1 1 1] Determine if hit piece should change colors. Delay put in place to allow proccessor to reset IsHit
  (bind _asbp_projectile_parent (cast `/Game/Projectiles/Blueprints/BP_ProjectileParent` OtherActor))
  (set `self.RefToProjectile` _asbp_projectile_parent)
  (`self.PuzzlePieceChangeColor` (`self.RefToProjectile`))
  (`KismetSystemLibrary.Delay` 0.01)
  (set `self.IsHit` false))

(fn `Change Color No Branch`
  (switch `/Game/GameValues/E_LightDark` (`self.LightDarkValue`)
    (:`NewEnumerator0`
      (`PrimitiveComponent.SetMaterial` (`self.StaticMesh`) 0 (`|GetArrayItem` (`self.Material`) 1))
      (set `self.LightDarkValue` "NewEnumerator1"))
    (:`NewEnumerator1`
      (`PrimitiveComponent.SetMaterial` (`self.StaticMesh`) 0 (`|GetArrayItem` (`self.Material`)))
      (set `self.LightDarkValue` "NewEnumerator0"))))

(fn `ChangeAdjacentPuzzlePiece`
  (params (TargetPuzzlePiece :type "/Game/Obstacles/Puzzle_01/BP_ColorPuzzleParent Object Reference"))
  (locals (CurrentPiece :type "/Game/Obstacles/Puzzle_01/BP_ColorPuzzleParent Object Reference"))
  (switch `/Game/GameValues/E_LightDark` (`/Game/Obstacles/Puzzle_01/BP_ColorPuzzleParent.LightDarkValue` TargetPuzzlePiece)
    (:`NewEnumerator0`
      (`PrimitiveComponent.SetMaterial` (`/Game/Obstacles/Puzzle_01/BP_ColorPuzzleParent.StaticMesh` (`local.TargetPuzzlePiece`)) 0 (`|GetArrayItem` (`self.Material`) 1))
      (set `self.LightDarkValue` "NewEnumerator1"))
    (:`NewEnumerator1`
      (`PrimitiveComponent.SetMaterial` (`/Game/Obstacles/Puzzle_01/BP_ColorPuzzleParent.StaticMesh` (`local.TargetPuzzlePiece`)) 0 (`|GetArrayItem` (`self.Material`)))
      (set `self.LightDarkValue` "NewEnumerator0"))))

(fn `PuzzlePieceChangeColor`
  (params (self2 :type "/Game/Projectiles/Blueprints/BP_ProjectileParent Object Reference"))
  (if (== (`/Game/Projectiles/Blueprints/BP_ProjectileParent.ProjectileValue` self2) (`self.LightDarkValue`))
    (set `self.IsHit` true)
    (`self.Change Color No Branch`)))

(fn `UserConstructionScript`)