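; Puzzle logic Blueprint for a five-piece light/dark puzzle that moves a wall when every piece shows the same value.
; BeginPlay caches the pieces from an array, then Tick polls the hit state of three of them, using DoOnce gates to change their linked pieces once per hit.
; Each Tick also compares the pieces' values against all-Light and all-Dark arrays, playing a timeline that shifts the wall's Z on a match.
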(event `self.ReceiveBeginPlay`
  ;[1 1 1] Set Puzzle Pieces to Different Values
  (`self.SetPuzzleTargets`))

(event `self.ReceiveTick`
  (params (DeltaSeconds :type "Float (single-precision)"))
  (`|ExecutionSequence`
    (:`then_0`
      ;[1 1 1] Determine Which pieces affect each other
      (`self.ChangeOneAdjacent`))
    (:`then_1`
      (`self.ChangeTwoAdjacent`))
    (:`then_2`
      (`self.ChangeThreeAdjacent`))
    (:`then_3`
      ;[1 1 1] Compare All values of puzzle and activate timeline if they are all identical
      (`self.CreateLightDarkValuesArray`)
      (bind _output_get (`self.AreAllValuesEqual`))
      (if _output_get
        (bind (_direction _movewallz) (`Timeline|MoveWallZ`)
          (:`Update`
            (`SceneComponent.K2_SetRelativeLocation` (`self.Wall`) (`KismetMathLibrary.MakeVector` 0.0 0.0 _movewallz) false false)))))))

(fn `AreAllValuesEqual`
  (returns (Output_Get :type Boolean))
  (bind _output_get (set `self.AreAllSame` (or (`KismetArrayLibrary.Array_Identical` (`self.LightDarkValues`) (`self.Light`)) (`KismetArrayLibrary.Array_Identical` (`self.LightDarkValues`) (`self.Dark`)))))
  (return _output_get))

(fn `ChangeOneAdjacent`
  (if (`/Game/Obstacles/Puzzle_01/BP_ColorPuzzleParent.IsHit` (`self.TargetPuzzlePiece_00`))
    (`/Engine/EditorBlueprintResources/StandardMacros.DoOnce` false :!label _label
      (:`Completed`
        (`/Game/Obstacles/Puzzle_01/BP_ColorPuzzleParent.ChangeAdjacentPuzzlePiece` (`self.TargetPuzzlePiece_01`) (`self.TargetPuzzlePiece_01`))))
    (else
      (goto _label :!via `Reset`))))

(fn `ChangeThreeAdjacent`
  (if (`/Game/Obstacles/Puzzle_01/BP_ColorPuzzleParent.IsHit` (`self.TargetPuzzlePiece_02`))
    (`/Engine/EditorBlueprintResources/StandardMacros.DoOnce` false :!label _label
      (:`Completed`
        (`/Game/Obstacles/Puzzle_01/BP_ColorPuzzleParent.ChangeAdjacentPuzzlePiece` (`self.TargetPuzzlePiece_00`) (`self.TargetPuzzlePiece_00`))
        (`/Game/Obstacles/Puzzle_01/BP_ColorPuzzleParent.ChangeAdjacentPuzzlePiece` (`self.TargetPuzzlePiece_03`) (`self.TargetPuzzlePiece_03`))
        (`/Game/Obstacles/Puzzle_01/BP_ColorPuzzleParent.ChangeAdjacentPuzzlePiece` (`self.TargetPuzzlePiece_04`) (`self.TargetPuzzlePiece_04`))))
    (else
      (goto _label :!via `Reset`))))

(fn `ChangeTwoAdjacent`
  (if (`/Game/Obstacles/Puzzle_01/BP_ColorPuzzleParent.IsHit` (`self.TargetPuzzlePiece_01`))
    (`/Engine/EditorBlueprintResources/StandardMacros.DoOnce` false :!label _label
      (:`Completed`
        (`/Game/Obstacles/Puzzle_01/BP_ColorPuzzleParent.ChangeAdjacentPuzzlePiece` (`self.TargetPuzzlePiece_02`) (`self.TargetPuzzlePiece_02`))
        (`/Game/Obstacles/Puzzle_01/BP_ColorPuzzleParent.ChangeAdjacentPuzzlePiece` (`self.TargetPuzzlePiece_03`) (`self.TargetPuzzlePiece_03`))))
    (else
      (goto _label :!via `Reset`))))

(fn `CreateLightDarkValuesArray`
  (set `self.LightDarkValues` (`|MakeArray` (`/Game/Obstacles/Puzzle_01/BP_ColorPuzzleParent.LightDarkValue` (`self.TargetPuzzlePiece_00`)) (`/Game/Obstacles/Puzzle_01/BP_ColorPuzzleParent.LightDarkValue` (`self.TargetPuzzlePiece_01`)) (`/Game/Obstacles/Puzzle_01/BP_ColorPuzzleParent.LightDarkValue` (`self.TargetPuzzlePiece_02`)) (`/Game/Obstacles/Puzzle_01/BP_ColorPuzzleParent.LightDarkValue` (`self.TargetPuzzlePiece_03`)) (`/Game/Obstacles/Puzzle_01/BP_ColorPuzzleParent.LightDarkValue` (`self.TargetPuzzlePiece_04`)))))

(fn `SetPuzzleTargets`
  (set `self.TargetPuzzlePiece_00` (`|GetArrayItem` (`self.PuzzlePieces`) (`self.PuzzlePiece_00`)))
  (set `self.TargetPuzzlePiece_01` (`|GetArrayItem` (`self.PuzzlePieces`) (`self.PuzzlePiece_01`)))
  (set `self.TargetPuzzlePiece_02` (`|GetArrayItem` (`self.PuzzlePieces`) (`self.PuzzlePiece_02`)))
  (set `self.TargetPuzzlePiece_03` (`|GetArrayItem` (`self.PuzzlePieces`) (`self.PuzzlePiece_03`)))
  (set `self.TargetPuzzlePiece_04` (`|GetArrayItem` (`self.PuzzlePieces`) (`self.PuzzlePiece_04`))))

(fn `UserConstructionScript`)