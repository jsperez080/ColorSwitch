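; Checkpoint actor that sets the player's respawn point and activates a child RespawnTotem_BP.
; Box overlap enables input and creates a press-E widget, shown only on first overlap because that overlap sets IsActive.
; Interaction stores the checkpoint as the player's CurrentCheckpoint and activates the totem; leaving removes the widget but keeps input enabled.
; A checkpoint flagged LevelBaseCheckpoint registers and activates itself on BeginPlay.
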(event `self.Box.OnComponentBeginOverlap`
  (params (OverlappedComponent :type "PrimitiveComponent Object Reference") (OtherActor :type "Actor Object Reference") (OtherComp :type "PrimitiveComponent Object Reference") (OtherBodyIndex :type Integer) (bFromSweep :type Boolean) (SweepResult :type "HitResult Structure (by ref)"))
  ;[1 1 1] Enable input if overlapped with player and display widget
  (cast `/Game/GameContent/PlayerCharacter/BP_PlayerCharacter` OtherActor)
  (`self.EnableInput` (`GameplayStatics.GetPlayerController` 0))
  (bind _returnvalue (`|CreateWidget` "/Game/GameContent/Obstacles/TeleportPuzzle/Switches/W_PressE.W_PressE_C"))
  (bind _output_get (set `self.PressEWidget` _returnvalue))
  (if (not (`self.IsActive`))
    (set `self.IsActive` true)
    (`UserWidget.AddToViewport` _output_get 0)))

(event `InputAction|InteractionButton`
  (params (Key :type "Key Structure"))
  ;[1 1 1] Activate Totem to set spawn point
  (:`Pressed`
    (bind _asbp_player_character (cast `/Game/GameContent/PlayerCharacter/BP_PlayerCharacter` (`GameplayStatics.GetPlayerPawn` 0)))
    (set `/Game/GameContent/PlayerCharacter/BP_PlayerCharacter.CurrentCheckpoint` self _asbp_player_character)
    (bind _asrespawn_totem_bp (cast `/Game/GameContent/models/RespawnTotem_BP` (`ChildActorComponent.ChildActor` (`self.RespawnTotem`))))
    (`/Game/GameContent/models/RespawnTotem_BP.ActivateTotem` _asrespawn_totem_bp)))

(event `self.Box.OnComponentEndOverlap`
  (params (OverlappedComponent :type "PrimitiveComponent Object Reference") (OtherActor :type "Actor Object Reference") (OtherComp :type "PrimitiveComponent Object Reference") (OtherBodyIndex :type Integer))
  ;[1 1 1] Remove widget when not overlapping
  (cast `/Game/GameContent/PlayerCharacter/BP_PlayerCharacter` OtherActor)
  (`Widget.RemoveFromParent` (`self.PressEWidget`)))

(event `self.ReceiveBeginPlay`
  (if (`self.LevelBaseCheckpoint`)
    (bind _asbp_player_character (cast `/Game/GameContent/PlayerCharacter/BP_PlayerCharacter` (`GameplayStatics.GetPlayerPawn` 0)))
    (set `/Game/GameContent/PlayerCharacter/BP_PlayerCharacter.CurrentCheckpoint` self _asbp_player_character)
    (bind _asrespawn_totem_bp (cast `/Game/GameContent/models/RespawnTotem_BP` (`ChildActorComponent.ChildActor` (`self.RespawnTotem`))))
    (set `self.IsActive` true)
    (`/Game/GameContent/models/RespawnTotem_BP.ActivateTotem` _asrespawn_totem_bp)))

(fn `UserConstructionScript`)