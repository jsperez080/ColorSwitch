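; Respawn totem actor that lights up and animates its floating top piece when ActivateTotem is called.
; Activation raises emissive intensity on base and top, then a timeline curve sets the top's hover height relative to the base.
; Each hover update also plays a second timeline that drives the top's yaw.
; The construction script creates dynamic material instances for both parts but neither stores nor assigns them.
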(event `ActivateTotem`
  (`MeshComponent.SetScalarParameterValueOnMaterials` (`self.RespawnTotemBase`) "Emissive Intensity" 1000.0)
  (`MeshComponent.SetScalarParameterValueOnMaterials` (`self.RespawnTotemTop`) "Emissive Intensity" 1000.0)
  (bind (_direction _tophovercurve) (`Timeline|RespawnTotemMovement`)
    (:`Update`
      (`SceneComponent.K2_SetWorldLocation` (`self.RespawnTotemTop`) (`KismetMathLibrary.MakeVector` (.x (`SceneComponent.K2_GetComponentLocation` (`self.RespawnTotemBase`))) (.y (`SceneComponent.K2_GetComponentLocation` (`self.RespawnTotemBase`))) (+ _tophovercurve (.z (`SceneComponent.K2_GetComponentLocation` (`self.RespawnTotemBase`))))) false false)
      (bind (_direction_2 _rotationcurve) (`Timeline|RespawnTotemRotation`)
        (:`Update`
          (`SceneComponent.K2_SetWorldRotation` (`self.RespawnTotemTop`) (`KismetMathLibrary.MakeRotator` 0.0 0.0 _rotationcurve) false false))))))

(fn `UserConstructionScript`
  (`KismetMaterialLibrary.CreateDynamicMaterialInstance` "/Game/GameContent/Materials/RespawnTotem/respawn_totem_top_MAT_Inst.respawn_totem_top_MAT_Inst")
  (`KismetMaterialLibrary.CreateDynamicMaterialInstance` "/Game/GameContent/Materials/RespawnTotem/respawn_totem_base_MAT_Inst.respawn_totem_base_MAT_Inst"))