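; One-shot crystal audio recording that the player triggers with an interact key after overlapping its sphere, which shows a press-E prompt.
; Chained timeline macros raise and tilt the crystal, split its halves, spin it while a 2D sound plays for AudioTime, then close and lower it.
; Construction caches the root's start transform, while Tick re-reads both halves' positions every frame, so split and collapse offsets apply to moving bases.
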(event `self.ReceiveBeginPlay`
  ;[1 1 1] Disable Rotator at start
  (`ActorComponent.SetActive` (`self.RotatingMovement`) false false))

(event `self.Sphere.OnComponentBeginOverlap`
  (params (OverlappedComponent :type "PrimitiveComponent Object Reference") (OtherActor :type "Actor Object Reference") (OtherComp :type "PrimitiveComponent Object Reference") (OtherBodyIndex :type Integer) (bFromSweep :type Boolean) (SweepResult :type "HitResult Structure (by ref)"))
  ;[1 1 1] Show Activate Widget when overlapped
  (cast `/Game/GameContent/PlayerCharacter/BP_PlayerCharacter` OtherActor)
  (if (not (`self.HasActivated`))
    (`self.EnableInput` (`GameplayStatics.GetPlayerController` 0))
    (bind _returnvalue (`|CreateWidget` "/Game/GameContent/Obstacles/TeleportPuzzle/Switches/W_PressE.W_PressE_C"))
    (bind _output_get (set `self.HUD_E` _returnvalue))
    (`UserWidget.AddToViewport` _output_get 0)))

(event `InputAction|InteractionButton`
  (params (Key :type "Key Structure"))
  (bind _crystalroot (`self.CrystalRoot`))
  ;[1 1 1] Play audio file if player has not activated it yet
  (:`Pressed`
    (if (not (`self.HasActivated`))
      (`/Engine/EditorBlueprintResources/StandardMacros.DoOnce` false
        (:`Completed`
          (set `self.HasActivated` true)
          (bind (_direction _fixrotation _setzlocation) (`Timeline|SetCrystalActive`)
            (:`Update`
              (`SceneComponent.K2_SetWorldLocationAndRotation` (`self.CrystalRoot`) (`KismetMathLibrary.MakeVector` (.x (`self.InitialLocation`)) (.y (`self.InitialLocation`)) (+ (.z (`self.InitialLocation`)) _setzlocation)) (`KismetMathLibrary.MakeRotator` (+ (.roll (`self.InitialRotation`)) _fixrotation) (.pitch (`self.InitialRotation`)) (.yaw (`self.InitialRotation`))) false false))
            (:`Finished`
              (`/Engine/EditorBlueprintResources/StandardMacros.DoOnce` false
                (:`Completed`
                  (`KismetSystemLibrary.Delay` 0.5)
                  (bind (_direction_2 _toploc _botloc) (`Timeline|BreakCrystal`)
                    (:`Update`
                      (`SceneComponent.K2_SetWorldLocation` (`self.CrystalTop`) (`KismetMathLibrary.MakeVector` (.x (`self.TopInitLoc`)) (.y (`self.TopInitLoc`)) (+ (.z (`self.TopInitLoc`)) _toploc)) false false)
                      (`SceneComponent.K2_SetWorldLocation` (`self.CrystalBottom`) (`KismetMathLibrary.MakeVector` (.x (`self.BotInitLoc`)) (.y (`self.BotInitLoc`)) (- (.z (`self.BotInitLoc`)) _botloc)) false false))
                    (:`Finished`
                      (`ActorComponent.SetActive` (`self.RotatingMovement`) true false)
                      (`GameplayStatics.PlaySound2D` (`self.AudioFile`) 1.0 1.0 0.0 null null)
                      (`KismetSystemLibrary.Delay` (`self.AudioTime`))
                      (`ActorComponent.SetActive` (`self.RotatingMovement`) false false)
                      (set `self.UpdatedCrystalLoc` (`SceneComponent.K2_GetComponentLocation` _crystalroot))
                      (set `self.UpdatedCrystalRot` (`SceneComponent.K2_GetComponentRotation` _crystalroot))
                      (bind (_direction_3 _toploc_2 _botloc_2) (`Timeline|CollapseCrystal`)
                        (:`Update`
                          (`SceneComponent.K2_SetWorldLocation` (`self.CrystalTop`) (`KismetMathLibrary.MakeVector` (.x (`self.TopInitLoc`)) (.y (`self.TopInitLoc`)) (- (.z (`self.TopInitLoc`)) _toploc_2)) false false)
                          (`SceneComponent.K2_SetWorldLocation` (`self.CrystalBottom`) (`KismetMathLibrary.MakeVector` (.x (`self.BotInitLoc`)) (.y (`self.BotInitLoc`)) (+ (.z (`self.BotInitLoc`)) _botloc_2)) false false))
                        (:`Finished`
                          (bind (_direction_4 _fixrotation_2 _setzlocation_2) (`Timeline|SetCrystalInactive`)
                            (:`Update`
                              (`SceneComponent.K2_SetWorldLocationAndRotation` (`self.CrystalRoot`) (`KismetMathLibrary.MakeVector` (.x (`self.UpdatedCrystalLoc`)) (.y (`self.UpdatedCrystalLoc`)) (- (.z (`self.UpdatedCrystalLoc`)) _setzlocation_2)) (`KismetMathLibrary.MakeRotator` (+ (.roll (`self.UpdatedCrystalRot`)) _fixrotation_2) (.pitch (`self.UpdatedCrystalRot`)) (.yaw (`self.UpdatedCrystalRot`))) false false))))))))))))))))

(event `self.Sphere.OnComponentEndOverlap`
  (params (OverlappedComponent :type "PrimitiveComponent Object Reference") (OtherActor :type "Actor Object Reference") (OtherComp :type "PrimitiveComponent Object Reference") (OtherBodyIndex :type Integer))
  ;[1 1 1] Remove widget when not overlapped
  (cast `/Game/GameContent/PlayerCharacter/BP_PlayerCharacter` OtherActor)
  (`Widget.RemoveFromParent` (`self.HUD_E`)))

(event `self.ReceiveTick`
  (params (DeltaSeconds :type "Float (single-precision)"))
  ;[1 1 1] Set individual component locations
  (set `self.TopInitLoc` (`SceneComponent.K2_GetComponentLocation` (`self.CrystalTop`)))
  (set `self.BotInitLoc` (`SceneComponent.K2_GetComponentLocation` (`self.CrystalBottom`))))

(fn `UserConstructionScript`
  (bind _crystalroot (`self.CrystalRoot`))
  (set `self.InitialLocation` (`SceneComponent.K2_GetComponentLocation` _crystalroot))
  (set `self.InitialRotation` (`SceneComponent.K2_GetComponentRotation` _crystalroot)))