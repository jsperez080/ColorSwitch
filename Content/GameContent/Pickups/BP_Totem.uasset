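; BP_Totem is a totem pickup that the player collects by overlapping it.
; On BeginPlay it finds and caches the level's BP_TeleportLogic actor.
; When a BP_PlayerCharacter enters its overlap component while that actor's AreAllRoomsActive is true, it adds itself to the player's Inventory under TotemName and destroys itself.
; The inventory receives a reference to the same actor that is then destroyed.
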(event `self.ReceiveBeginPlay`
  (bind _returnvalue (`GameplayStatics.GetActorOfClass` "/Game/GameContent/Obstacles/TeleportPuzzle/BP_TeleportLogic.BP_TeleportLogic_C"))
  (set `self.TeleporterLogic` _returnvalue))

(event `self.Overlap.OnComponentBeginOverlap`
  (params (OverlappedComponent :type "PrimitiveComponent Object Reference") (OtherActor :type "Actor Object Reference") (OtherComp :type "PrimitiveComponent Object Reference") (OtherBodyIndex :type Integer) (bFromSweep :type Boolean) (SweepResult :type "HitResult Structure (by ref)"))
  ;[1 1 1] Pickup totem and add to player inventory upon overlap
  (bind _asbp_player_character (cast `/Game/GameContent/PlayerCharacter/BP_PlayerCharacter` OtherActor))
  (if (`/Game/GameContent/Obstacles/TeleportPuzzle/BP_TeleportLogic.AreAllRoomsActive` (`self.TeleporterLogic`))
    (`BlueprintMapLibrary.Map_Add` (`/Game/GameContent/PlayerCharacter/BP_PlayerCharacter.Inventory` _asbp_player_character) (`self.TotemName`) self)
    (`self.K2_DestroyActor`)))

(fn `UserConstructionScript`)