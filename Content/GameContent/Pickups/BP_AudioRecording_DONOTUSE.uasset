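; Audio recording pickup (named DONOTUSE) that plays its sound once when the player presses the interaction button.
; Sphere overlap enables input and shows a press-E widget until activated; leaving removes the widget but not input.
; A timeline moves and tilts the device from its construction-time transform, then rotation and 2D audio start.
; After the AudioTime delay, rotation stops and the timeline reverses, with DoOnce blocking a replay on finish.
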(event `self.ReceiveBeginPlay`
  ;[1 1 1] Disable Rotator at start
  (`ActorComponent.SetActive` (`self.RotatingMovement`) false false))

(event `self.Sphere.OnComponentBeginOverlap`
  (params (OverlappedComponent :type "PrimitiveComponent Object Reference") (OtherActor :type "Actor Object Reference") (OtherComp :type "PrimitiveComponent Object Reference") (OtherBodyIndex :type Integer) (bFromSweep :type Boolean) (SweepResult :type "HitResult Structure (by ref)"))
  ;[1 1 1] Show Activate Widget when overlapped
  (cast `/Game/GameContent/PlayerCharacter/BP_PlayerCharacter` OtherActor)
  (if (not (`self.HasActivated`))
    (`self.EnableInput` (`GameplayStatics.GetPlayerController` 0))
    (bind _returnvalue (`|CreateWidget` "/Game/GameContent/Obstacles/TeleportPuzzle/Switches/W_PressE.W_PressE_C"))
    (bind _output_get (set `self.HUD_E` _returnvalue))
    (`UserWidget.AddToViewport` _output_get 0)))

(event `InputAction|InteractionButton`
  (params (Key :type "Key Structure"))
  ;[1 1 1] Play audio file if player has not activated it yet
  (:`Pressed`
    (if (not (`self.HasActivated`))
      (`/Engine/EditorBlueprintResources/StandardMacros.DoOnce` false
        (:`Completed`
          (set `self.HasActivated` true)
          (bind (_direction _fixrotation _setzlocation) (`Timeline|SetCrystalActive` :!label _label)
            (:`Update`
              (`SceneComponent.K2_SetWorldLocationAndRotation` (`self.RecordingDevice`) (`KismetMathLibrary.MakeVector` (.x (`self.InitialLocation`)) (.y (`self.InitialLocation`)) (+ (.z (`self.InitialLocation`)) _setzlocation)) (`KismetMathLibrary.MakeRotator` (+ (.roll (`self.InitialRotation`)) _fixrotation) (.pitch (`self.InitialRotation`)) (.yaw (`self.InitialRotation`))) false false))
            (:`Finished`
              (`/Engine/EditorBlueprintResources/StandardMacros.DoOnce` false
                (:`Completed`
                  (`KismetSystemLibrary.Delay` 0.2)
                  (`ActorComponent.SetActive` (`self.RotatingMovement`) true false)
                  (`GameplayStatics.PlaySound2D` (`self.AudioFile`) 1.0 1.0 0.0 null null)
                  (`KismetSystemLibrary.Delay` (`self.AudioTime`))
                  (`ActorComponent.SetActive` (`self.RotatingMovement`) false false)
                  (goto _label :!via `Reverse`))))))))))

(event `self.Sphere.OnComponentEndOverlap`
  (params (OverlappedComponent :type "PrimitiveComponent Object Reference") (OtherActor :type "Actor Object Reference") (OtherComp :type "PrimitiveComponent Object Reference") (OtherBodyIndex :type Integer))
  ;[1 1 1] Remove widget when not overlapped
  (cast `/Game/GameContent/PlayerCharacter/BP_PlayerCharacter` OtherActor)
  (`Widget.RemoveFromParent` (`self.HUD_E`)))

(fn `UserConstructionScript`
  (bind _recordingdevice (`self.RecordingDevice`))
  (set `self.InitialLocation` (`SceneComponent.K2_GetComponentLocation` _recordingdevice))
  (set `self.InitialRotation` (`SceneComponent.K2_GetComponentRotation` _recordingdevice)))