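; BP_Enemy is an AI enemy that senses targets through AI perception and tracks the last perceived actor.
; On sighting, it cancels the lost-target timer and passes the target, player and line-of-sight keys to its BP_AIC_Enemy controller.
; On losing sight, it clears line of sight immediately and starts a five-second timer, after which TargetLost forgets the actor and resets the target and player keys.
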(event `self.AIPerception.OnTargetPerceptionUpdated`
  (params (Actor :type "Actor Object Reference") (Stimulus :type "AIStimulus Structure"))
  ;[1 1 1] When target is sighted and AI loses sight, call TargetLost event. If target is still sensed then clear timer of event.
  ;;[1 1 1] Is the target sensed the character AI wishes to pursue?
  (set `self.PerceivedActor` Actor)
  (if (`.bSuccessfullySensed` (break `AIStimulus` Stimulus))
    ;;[1 1 1] Still in sight = keep interest in target
    (`KismetSystemLibrary.K2_ClearAndInvalidateTimerHandle` (`self.TargetLostTimer`))
    (`/Game/GameContent/AI/Enemy/EnemyandController/BP_AIC_Enemy.HasTargetActorKey` (`self.GetAIController`) (`self.PerceivedActor`))
    (`/Game/GameContent/AI/Enemy/EnemyandController/BP_AIC_Enemy.HasLineOfSightKey` (`self.GetAIController`) true)
    (`/Game/GameContent/AI/Enemy/EnemyandController/BP_AIC_Enemy.HasPlayerActorKey` (`self.GetAIController`) (`self.PerceivedActor`))
    (else
      ;;[1 1 1] Lost sight = lose interest
      (bind _returnvalue (`KismetSystemLibrary.K2_SetTimerDelegate` (delegate `TargetLost`) 5.0))
      (set `self.TargetLostTimer` _returnvalue)
      (`/Game/GameContent/AI/Enemy/EnemyandController/BP_AIC_Enemy.HasLineOfSightKey` (`self.GetAIController`) false))))

(event `TargetLost`
  ;[1 1 1] When target is sighted and AI loses sight, call TargetLost event. If target is still sensed then clear timer of event.
  ;;[1 1 1] Lost sight = lose interest
  (set `self.PerceivedActor` null)
  (`/Game/GameContent/AI/Enemy/EnemyandController/BP_AIC_Enemy.HasTargetActorKey` (`self.GetAIController`) null)
  (`/Game/GameContent/AI/Enemy/EnemyandController/BP_AIC_Enemy.HasPlayerActorKey` (`self.GetAIController`) null))

(fn `GetAIController`
  (returns (`AsBP AIC Enemy` :type "/Game/GameContent/AI/Enemy/EnemyandController/BP_AIC_Enemy Object Reference"))
  (return (cast `/Game/GameContent/AI/Enemy/EnemyandController/BP_AIC_Enemy` (`self.GetController`) :!pure true)))

(fn `UserConstructionScript`)