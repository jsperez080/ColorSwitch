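; Slug enemy character that senses targets and fires projectiles at the player.
; Tick checks player distance and, unless the attack montage is playing, turns to face, plays it and spawns a projectile aimed via line trace.
; AI Perception feeds target and line-of-sight keys to BP_AIC_Slug, clearing the target through a five-second timer after sight loss.
; Projectile hits reduce health; a hit at zero health destroys the slug.
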(event `self.ReceiveBeginPlay`
  ;[1 1 1] Set Slug Speed
  (set `CharacterMovementComponent.MaxWalkSpeed` (`self.SlugSpeed`) (`self.CharacterMovement`)))

(event `self.ReceiveTick`
  (params (DeltaSeconds :type "Float (single-precision)"))
  ;[1 1 1] Attack Player if In Range
  (if (`self.IsWithinAttackRange`)
    (if (not (`self.IsAttacking`))
      (`self.RotateActorLookAT`)
      (`|PlayMontage` (`self.Mesh`) "/Game/GameContent/models/Snail/Slug_Attack.Slug_Attack"
        (:`then`
          (`self.SpawnProjectile`))))))

(event `self.AIPerception.OnTargetPerceptionUpdated`
  (params (Actor :type "Actor Object Reference") (Stimulus :type "AIStimulus Structure"))
  ;[1 1 1] When target is sighted and AI loses sight, call TargetLost event. If target is still sensed then clear timer of event.
  ;;[1 1 1] Is the target sensed the character AI wishes to pursue?
  (set `self.PerceivedActor` Actor)
  (if (`.bSuccessfullySensed` (break `AIStimulus` Stimulus))
    ;;[1 1 1] Still in sight = keep interest in target
    (`KismetSystemLibrary.K2_ClearAndInvalidateTimerHandle` (`self.TargetLostTimer`))
    (`/Game/GameContent/AI/Enemy/Slug/BP_AIC_Slug.HasTargetActorKey` (`self.GetAIController`) (`self.PerceivedActor`))
    (`/Game/GameContent/AI/Enemy/Slug/BP_AIC_Slug.HasLineOfSightKey` (`self.GetAIController`) true)
    (`/Game/GameContent/AI/Enemy/Slug/BP_AIC_Slug.HasPlayerActorKey` (`self.GetAIController`) (`self.PerceivedActor`))
    (else
      ;;[1 1 1] Lost sight = lose interest
      (bind _returnvalue (`KismetSystemLibrary.K2_SetTimerDelegate` (delegate `TargetLost`) 5.0))
      (set `self.TargetLostTimer` _returnvalue)
      (`/Game/GameContent/AI/Enemy/Slug/BP_AIC_Slug.HasLineOfSightKey` (`self.GetAIController`) false))))

(event `TargetLost`
  ;[1 1 1] When target is sighted and AI loses sight, call TargetLost event. If target is still sensed then clear timer of event.
  ;;[1 1 1] Lost sight = lose interest
  (set `self.PerceivedActor` null)
  (`/Game/GameContent/AI/Enemy/Slug/BP_AIC_Slug.HasTargetActorKey` (`self.GetAIController`) null)
  (`/Game/GameContent/AI/Enemy/Slug/BP_AIC_Slug.HasPlayerActorKey` (`self.GetAIController`) null))

(event `self.ReceiveHit`
  (params (MyComp :type "PrimitiveComponent Object Reference") (Other :type "Actor Object Reference") (OtherComp :type "PrimitiveComponent Object Reference") (bSelfMoved :type Boolean) (HitLocation :type "Vector Structure") (HitNormal :type "Vector Structure") (NormalImpulse :type "Vector Structure") (Hit :type "HitResult Structure (by ref)"))
  ;[1 1 1] Lower Slug Health if hit
  (bind _asbp_projectile_parent (cast `/Game/GameContent/Projectiles/Blueprints/PlayerProjectile/BP_ProjectileParent` Other))
  (if (<= (`self.Health`) 0.0)
    (`self.K2_DestroyActor`)
    (else
      (set `self.Health` (`KismetMathLibrary.FMax` (- (`self.Health`) (`/Game/GameContent/Projectiles/Blueprints/PlayerProjectile/BP_ProjectileParent.ProjectileDamage` _asbp_projectile_parent)))))))

(fn `GetAIController`
  (returns (`AsBP AIC Slug` :type "/Game/GameContent/AI/Enemy/Slug/BP_AIC_Slug Object Reference"))
  (return (cast `/Game/GameContent/AI/Enemy/Slug/BP_AIC_Slug` (`self.GetController`) :!pure true)))

(fn `IsAttacking`
  (returns (ReturnValue :type Boolean))
  (return (`AnimInstance.Montage_IsPlaying` (`SkeletalMeshComponent.GetAnimInstance` (`self.Mesh`)) "/Game/GameContent/models/Snail/Slug_Attack.Slug_Attack")))

(fn `IsWithinAttackRange`
  (returns (ReturnValue :type Boolean))
  (return (< (`self.GetDistanceTo` (`GameplayStatics.GetPlayerCharacter` 0)) (`self.AttackRange`))))

(fn `RotateActorLookAT`
  (`self.K2_SetActorRotation` (`KismetMathLibrary.FindLookAtRotation` (`SceneComponent.K2_GetComponentLocation` (`self.Mesh`)) (`SceneComponent.K2_GetComponentLocation` (`Character.CapsuleComponent` (`GameplayStatics.GetPlayerCharacter` 0))))))

(fn `SpawnProjectile`
  (bind _returnvalue (`SceneComponent.K2_GetComponentLocation` (`self.SpawnPoint`)))
  (bind (_outhit _returnvalue_2) (`KismetSystemLibrary.LineTraceSingle` (`SceneComponent.K2_GetComponentLocation` (`self.SpawnPoint`)) (`SceneComponent.K2_GetComponentLocation` (`Character.CapsuleComponent` (`GameplayStatics.GetPlayerCharacter` 0))) "TraceTypeQuery1" false (`|MakeArray` self)))
  (bind (_bblockinghit _binitialoverlap _time _distance _location _impactpoint _normal _impactnormal _physmat _hitactor _hitcomponent _hitbonename _hititem _faceindex _tracestart _traceend) (`GameplayStatics.BreakHitResult` _outhit))
  (`|SpawnActorFromClass` "/Game/GameContent/Projectiles/Blueprints/SlugProjectiles/BP_SlugProjectile.BP_SlugProjectile_C" (`KismetMathLibrary.MakeTransform` _returnvalue (`KismetMathLibrary.FindLookAtRotation` _returnvalue (`KismetMathLibrary.SelectVector` _impactpoint _traceend _returnvalue_2))) "AlwaysSpawn" "OverrideRootScale" null null))

(fn `UserConstructionScript`)