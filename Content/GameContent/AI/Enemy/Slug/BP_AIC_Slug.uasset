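; AI controller for the Slug enemy that runs the BT_Enemy behavior tree on possess.
; Setter functions write Blackboard values for the target actor, the player (cast to BP_PlayerCharacter) and a patrol location.
; The patrol setter stores the location of a randomly chosen actor from the supplied array.
; The line-of-sight setter writes its bool to a key named "None".
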(event `self.ReceivePossess`
  (params (PossessedPawn :type "Pawn Object Reference"))
  (`self.RunBehaviorTree` "/Game/GameContent/AI/Enemy/BehaviorTree/BT_Enemy.BT_Enemy"))

(fn `HasLineOfSightKey`
  (params (HasLineOfSight :type Boolean))
  (`BlackboardComponent.SetValueAsBool` (`AIBlueprintHelperLibrary.GetBlackboard` null) "None" HasLineOfSight))

(fn `HasPatrolPointKey`
  (params (PatrolLocationKey :type "Array of TargetPoint Object Reference"))
  (`BlackboardComponent.SetValueAsVector` (`AIBlueprintHelperLibrary.GetBlackboard` null) "PatrolLocation" (`self.K2_GetActorLocation` (`|GetArrayItem` PatrolLocationKey (`KismetMathLibrary.RandomInteger` (`KismetArrayLibrary.Array_Length` PatrolLocationKey))))))

(fn `HasPlayerActorKey`
  (params (PlayerActor :type "Actor Object Reference"))
  (bind _asbp_player_character (cast `/Game/GameContent/PlayerCharacter/BP_PlayerCharacter` PlayerActor))
  (`BlackboardComponent.SetValueAsObject` (`AIBlueprintHelperLibrary.GetBlackboard` null) "PlayerActor" _asbp_player_character))

(fn `HasTargetActorKey`
  (params (TargetActor :type "Actor Object Reference"))
  (`BlackboardComponent.SetValueAsObject` (`AIBlueprintHelperLibrary.GetBlackboard` null) "TargetActor" TargetActor))

(fn `UserConstructionScript`)