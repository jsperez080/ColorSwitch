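; BP_MovementLogic is the movement puzzle controller that moves itself vertically as a wall once every platform is active.
; On BeginPlay it gathers all BP_PlatformParent actors in the level, then checks their IsActive flags each Tick through a Gate.
; When all are active, a DoOnce plays the MoveWall timeline, which sets the actor's world Z directly and closes the Gate to stop further checks.
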(event `self.ReceiveBeginPlay`
  (bind _outactors (`GameplayStatics.GetAllActorsOfClass` "/Game/GameContent/Obstacles/MovementPuzzle/TriggerPlatforms/BP_PlatformParent.BP_PlatformParent_C"))
  (set `self.TriggerValues` _outactors))

(event `self.ReceiveTick`
  (params (DeltaSeconds :type "Float (single-precision)"))
  (`/Engine/EditorBlueprintResources/StandardMacros.Gate` false :!label _label
    (:`Exit`
      (bind _alltrue (`self.AreAllPlatformsActive`))
      (bind _output_get (set `self.AllActive` _alltrue))
      (if _output_get
        (`/Engine/EditorBlueprintResources/StandardMacros.DoOnce` false
          (:`Completed`
            (bind (_direction _zwallmove) (`Timeline|MoveWall`)
              (:`Update`
                (`self.K2_SetActorLocation` (`KismetMathLibrary.MakeVector` (.x (`self.K2_GetActorLocation`)) (.y (`self.K2_GetActorLocation`)) _zwallmove))
                (goto _label :!via `Close`)))))))))

(fn `AreAllPlatformsActive`
  (returns (AllTrue :type Boolean))
  (for _array_element (`self.TriggerValues`)
    (if (not (`/Game/GameContent/Obstacles/MovementPuzzle/TriggerPlatforms/BP_PlatformParent.IsActive` _array_element))
      (return false)))
  (return true))

(fn `UserConstructionScript`)