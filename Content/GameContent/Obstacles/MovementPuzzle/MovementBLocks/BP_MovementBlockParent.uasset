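; BP_MovementBlockParent is a movement puzzle block that only a projectile with a matching light/dark value can push.
; On a component hit, it compares the projectile's value to its own, then enables physics and applies a velocity-change impulse.
; The impulse direction comes from a look-at rotation between projectile location and impact normal, with the normal used as a target position.
; Any non-projectile hit switches physics off again.
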(event `self.Block.OnComponentHit`
  (params (HitComponent :type "PrimitiveComponent Object Reference") (OtherActor :type "Actor Object Reference") (OtherComp :type "PrimitiveComponent Object Reference") (NormalImpulse :type "Vector Structure") (Hit :type "HitResult Structure (by ref)"))
  ;[1 1 1] Enable Physics only when hit with correct projectile
  (bind _asbp_projectile_parent (cast `/Game/GameContent/Projectiles/Blueprints/BP_ProjectileParent` OtherActor)
    (:`then`
      (set `self.CanMove` true)
      (if (and (`|EnumEquality` (`/Game/GameContent/Projectiles/Blueprints/BP_ProjectileParent.ProjectileValue` _asbp_projectile_parent) (`self.LightDarkValue`)) (`self.CanMove`))
        (`PrimitiveComponent.SetSimulatePhysics` (`self.Block`) true)
        (`PrimitiveComponent.AddImpulse` (`self.Block`) (* (`KismetMathLibrary.GetForwardVector` (`KismetMathLibrary.FindLookAtRotation` (`self.K2_GetActorLocation` _asbp_projectile_parent) (`.ImpactNormal` (`GameplayStatics.BreakHitResult` Hit)))) 1000.0) "None" true)))
    (:`CastFailed`
      (set `self.CanMove` false)
      (`PrimitiveComponent.SetSimulatePhysics` (`self.Block`) false))))

(fn `UserConstructionScript`)