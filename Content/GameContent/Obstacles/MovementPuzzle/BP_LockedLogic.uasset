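; BP_LockedLogic is a movement-puzzle obstacle, a wall that lowers when its linked triggers are active.
; Every Tick it queries AreAllPlatformsActive, playing the MoveWall timeline when true and reversing it otherwise; Finished re-runs the check.
; The timeline subtracts its Z offset from the location cached in the construction script.
; Despite its name, AreAllPlatformsActive returns on the first TriggerValues element, so only that trigger decides.
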(event `self.ReceiveTick`
  (params (DeltaSeconds :type "Float (single-precision)"))
  ;[1 1 1] Open or close lock based on overlapping actor
  (bind _alltrue (`self.AreAllPlatformsActive` :!label _label))
  (bind _output_get (set `self.AllActive` _alltrue))
  (if _output_get
    (bind (_direction _zwallmove) (`Timeline|MoveWall` :!label _label_2)
      (:`Update`
        (`self.K2_SetActorLocation` (`KismetMathLibrary.MakeVector` (.x (`self.InitialLocation`)) (.y (`self.InitialLocation`)) (- (.z (`self.InitialLocation`)) _zwallmove))))
      (:`Finished`
        (goto _label)))
    (else
      (goto _label_2 :!via `Reverse`))))

(fn `AreAllPlatformsActive`
  (returns (AllTrue :type Boolean))
  (for _array_element (`self.TriggerValues`)
    (if (`/Game/GameContent/Obstacles/MovementPuzzle/TriggerPlatforms/BP_PlatformParent.IsActive` _array_element)
      (return true)
      (else
        (return false)))))

(fn `UserConstructionScript`
  (set `self.InitialLocation` (`self.K2_GetActorLocation`)))