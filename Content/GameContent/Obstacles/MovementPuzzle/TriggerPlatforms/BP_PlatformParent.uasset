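; Parent pressure-platform Blueprint for a movement puzzle that sinks when a movement block with a matching LightDarkValue enters its box.
; The DepressBlock timeline lowers the actor along Z from the transform cached in the construction script, setting IsActive as it updates.
; A mismatched block reverses the timeline only while inactive.
; Ending any overlap clears IsActive without raising the platform.
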(event `self.Box.OnComponentBeginOverlap`
  (params (OverlappedComponent :type "PrimitiveComponent Object Reference") (OtherActor :type "Actor Object Reference") (OtherComp :type "PrimitiveComponent Object Reference") (OtherBodyIndex :type Integer) (bFromSweep :type Boolean) (SweepResult :type "HitResult Structure (by ref)"))
  (bind _asbp_movement_block_parent (cast `/Game/GameContent/Obstacles/MovementPuzzle/MovementBLocks/BP_MovementBlockParent` OtherActor))
  (if (`|EnumEquality` (`/Game/GameContent/Obstacles/MovementPuzzle/MovementBLocks/BP_MovementBlockParent.LightDarkValue` _asbp_movement_block_parent) (`self.LightDarkValue`))
    (bind (_direction _zdepress) (`Timeline|DepressBlock` :!label _label)
      (:`Update`
        (`self.K2_SetActorLocation` (`KismetMathLibrary.MakeVector` (.x (.location (`self.InitialTransform`))) (.y (.location (`self.InitialTransform`))) (- (.z (.location (`self.InitialTransform`))) _zdepress)))
        (set `self.IsActive` true)))
    (elif (not (`self.IsActive`))
      (goto _label :!via `Reverse`))))

(event `self.Box.OnComponentEndOverlap`
  (params (OverlappedComponent :type "PrimitiveComponent Object Reference") (OtherActor :type "Actor Object Reference") (OtherComp :type "PrimitiveComponent Object Reference") (OtherBodyIndex :type Integer))
  (set `self.IsActive` false))

(fn `UserConstructionScript`
  (set `self.InitialTransform` (`self.GetTransform`)))