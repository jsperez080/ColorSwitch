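; Obstacle platform with ten guard pieces that rotate out of position when a BP_DarkProjectile hits its base.
; A hit starts a music cue and a timeline that tilts each guard from its BeginPlay rotation while animating the base's dynamic material color and emissive.
; Five seconds after the timeline finishes, the sound toggles and the hit lock clears.
; Tick continually adds yaw to the guards; the player overlap sphere is an unimplemented stub.
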(event `self.PlatformBase.OnComponentHit`
  (params (HitComponent :type "PrimitiveComponent Object Reference") (OtherActor :type "Actor Object Reference") (OtherComp :type "PrimitiveComponent Object Reference") (NormalImpulse :type "Vector Structure") (Hit :type "HitResult Structure (by ref)"))
  ;[1 1 1] PFG Functions
  (cast `/Game/GameContent/Projectiles/Blueprints/BP_DarkProjectile` OtherActor)
  (if (not (`self.PlatformGuardDown`))
    (set `self.PlatformGuardDown` true)
    (if (not (`self.Sound Active`))
      (bind _returnvalue (`GameplayStatics.SpawnSound2D` "/Game/StarterContent/Audio/Starter_Music_Cue.Starter_Music_Cue" 1.0 1.0 0.0 null)))
    (`ActorComponent.SetActive` _returnvalue true false)
    (set `self.Sound Active` true)
    (bind (_direction _rotation_curve _emissive_color _color) (`Timeline|RotationTimeLine`)
      (:`Update`
        ;;[1 1 1] PFG1,4,6,9
        (`SceneComponent.K2_SetRelativeRotation` (`self.PFG1`) (`KismetMathLibrary.MakeRotator` (.roll (`self.Initial PFG1 Rotation`)) (+ (.pitch (`self.Initial PFG1 Rotation`)) _rotation_curve) (.yaw (`self.Initial PFG1 Rotation`))) false false)
        (`SceneComponent.K2_SetRelativeRotation` (`self.PFG4`) (`KismetMathLibrary.MakeRotator` (+ (.roll (`self.Initial PFG4 Rotation`)) _rotation_curve) (.pitch (`self.Initial PFG4 Rotation`)) (.yaw (`self.Initial PFG4 Rotation`))) false false)
        (`SceneComponent.K2_SetRelativeRotation` (`self.PFG6`) (`KismetMathLibrary.MakeRotator` (.roll (`self.Initial PFG6 Rotation`)) (* -1.0 (+ (.pitch (`self.Initial PFG6 Rotation`)) _rotation_curve)) (.yaw (`self.Initial PFG6 Rotation`))) false false)
        (`SceneComponent.K2_SetRelativeRotation` (`self.PFG9`) (`KismetMathLibrary.MakeRotator` (* -1.0 (+ (.roll (`self.Initial PFG9 Rotatio`)) _rotation_curve)) (.pitch (`self.Initial PFG9 Rotatio`)) (.yaw (`self.Initial PFG9 Rotatio`))) false false)
        ;;[1 1 1] PFG2,3,7,8
        (`SceneComponent.K2_SetRelativeRotation` (`self.PFG2`) (`KismetMathLibrary.MakeRotator` (.roll (`self.Initial PFG2 Rotation`)) (+ (.pitch (`self.Initial PFG2 Rotation`)) _rotation_curve) (.yaw (`self.Initial PFG2 Rotation`))) false false)
        (`SceneComponent.K2_SetRelativeRotation` (`self.PFG3`) (`KismetMathLibrary.MakeRotator` (+ (.roll (`self.Initial PFG3 Rotation`)) _rotation_curve) (.pitch (`self.Initial PFG3 Rotation`)) (.yaw (`self.Initial PFG3 Rotation`))) false false)
        (`SceneComponent.K2_SetRelativeRotation` (`self.PFG7`) (`KismetMathLibrary.MakeRotator` (.roll (`self.Initial PFG7 Rotatio`)) (* (+ (.pitch (`self.Initial PFG7 Rotatio`)) _rotation_curve) -1.0) (.yaw (`self.Initial PFG7 Rotatio`))) false false)
        (`SceneComponent.K2_SetRelativeRotation` (`self.PFG8`) (`KismetMathLibrary.MakeRotator` (* -1.0 (+ (.roll (`self.Initial PFG8 Rotatio`)) _rotation_curve)) (.pitch (`self.Initial PFG8 Rotatio`)) (.yaw (`self.Initial PFG8 Rotatio`))) false false)
        ;;[1 1 1] PFG5,10
        (`SceneComponent.K2_SetRelativeRotation` (`self.PFG5`) (`KismetMathLibrary.MakeRotator` (+ (.roll (`self.Initial PFG5 Rotation`)) _rotation_curve) (* -0.7 (+ (.pitch (`self.Initial PFG5 Rotation`)) _rotation_curve)) (.yaw (`self.Initial PFG5 Rotation`))) false false)
        (`SceneComponent.K2_SetRelativeRotation` (`self.PFG10`) (`KismetMathLibrary.MakeRotator` (* -0.7 (+ (.roll (`self.Initial PFG10 Rotatio`)) _rotation_curve)) (+ (.pitch (`self.Initial PFG10 Rotatio`)) _rotation_curve) (.yaw (`self.Initial PFG10 Rotatio`))) false false)
        ;[1 1 1] Dynamic Materials
        (`MaterialInstanceDynamic.SetVectorParameterValue` (stale `self.ReceiveBeginPlay` _returnvalue) "Color" _color)
        (`MaterialInstanceDynamic.SetScalarParameterValue` (stale `self.ReceiveBeginPlay` _returnvalue) "Emissive Color" _emissive_color))
      (:`Finished`
        (`KismetSystemLibrary.Delay` 5.0)
        (`ActorComponent.ToggleActive` _returnvalue)
        (set `self.Sound Active` false)
        (set `self.PlatformGuardDown` false)))))

(event `self.Sphere.OnComponentBeginOverlap`
  (params (OverlappedComponent :type "PrimitiveComponent Object Reference") (OtherActor :type "Actor Object Reference") (OtherComp :type "PrimitiveComponent Object Reference") (OtherBodyIndex :type Integer) (bFromSweep :type Boolean) (SweepResult :type "HitResult Structure (by ref)"))
  ;[1 1 1] PFG Functions
  ;;[1 1 1] For further implementation.
  (cast `/Game/GameContent/PlayerCharacter/BP_PlayerCharacter` OtherActor))

(event `self.ReceiveBeginPlay`
  ;[1 1 1] Getting Initial Rotations of all the platform guards.
  (set `self.Initial PFG1 Rotation` (`SceneComponent.K2_GetComponentRotation` (`self.PFG1`)))
  (set `self.Initial PFG2 Rotation` (`SceneComponent.K2_GetComponentRotation` (`self.PFG2`)))
  (set `self.Initial PFG3 Rotation` (`SceneComponent.K2_GetComponentRotation` (`self.PFG3`)))
  (set `self.Initial PFG4 Rotation` (`SceneComponent.K2_GetComponentRotation` (`self.PFG4`)))
  (set `self.Initial PFG5 Rotation` (`SceneComponent.K2_GetComponentRotation` (`self.PFG5`)))
  (set `self.Initial PFG6 Rotation` (`SceneComponent.K2_GetComponentRotation` (`self.PFG6`)))
  (set `self.Initial PFG7 Rotatio` (`SceneComponent.K2_GetComponentRotation` (`self.PFG7`)))
  (set `self.Initial PFG8 Rotatio` (`SceneComponent.K2_GetComponentRotation` (`self.PFG8`)))
  (set `self.Initial PFG9 Rotatio` (`SceneComponent.K2_GetComponentRotation` (`self.PFG9`)))
  (set `self.Initial PFG10 Rotatio` (`SceneComponent.K2_GetComponentRotation` (`self.PFG10`)))
  ;[1 1 1] Dynamic Materials
  (bind _returnvalue (`PrimitiveComponent.CreateDynamicMaterialInstance` (`self.PlatformBase`) 0 "/Game/GameContent/Obstacles/DynamicPlatform/Blueprints/BlueprintsForPlatform/Mesh/Materials/M_Platform.M_Platform" "None")))

(event `self.ReceiveTick`
  (params (DeltaSeconds :type "Float (single-precision)"))
  ;[1 1 1] Rotation Handler
  (`SceneComponent.K2_AddRelativeRotation` (`self.PFG1`) (`KismetMathLibrary.MakeRotator` 0.0 0.0 (* DeltaSeconds (`self.RotationMultiplier`))) false false)
  (`SceneComponent.K2_AddRelativeRotation` (`self.PFG2`) (`KismetMathLibrary.MakeRotator` 0.0 0.0 (* DeltaSeconds (`self.RotationMultiplier`))) false false)
  (`SceneComponent.K2_AddRelativeRotation` (`self.PFG3`) (`KismetMathLibrary.MakeRotator` 0.0 0.0 (* DeltaSeconds (`self.RotationMultiplier`))) false false)
  (`SceneComponent.K2_AddRelativeRotation` (`self.PFG4`) (`KismetMathLibrary.MakeRotator` 0.0 0.0 (* DeltaSeconds (`self.RotationMultiplier`))) false false)
  (`SceneComponent.K2_AddRelativeRotation` (`self.PFG5`) (`KismetMathLibrary.MakeRotator` 0.0 0.0 (* DeltaSeconds (`self.RotationMultiplier`))) false false)
  (`SceneComponent.K2_AddRelativeRotation` (`self.PFG6`) (`KismetMathLibrary.MakeRotator` 0.0 0.0 (* DeltaSeconds (`self.RotationMultiplier`))) false false)
  (`SceneComponent.K2_AddRelativeRotation` (`self.PFG7`) (`KismetMathLibrary.MakeRotator` 0.0 0.0 (* DeltaSeconds (`self.RotationMultiplier`))) false false)
  (`SceneComponent.K2_AddRelativeRotation` (`self.PFG8`) (`KismetMathLibrary.MakeRotator` 0.0 0.0 (* DeltaSeconds (`self.RotationMultiplier`))) false false)
  (`SceneComponent.K2_AddRelativeRotation` (`self.PFG9`) (`KismetMathLibrary.MakeRotator` 0.0 0.0 (* DeltaSeconds (`self.RotationMultiplier`))) false false)
  (`SceneComponent.K2_AddRelativeRotation` (`self.PFG10`) (`KismetMathLibrary.MakeRotator` 0.0 0.0 (* DeltaSeconds (`self.RotationMultiplier`))) false false))

(fn `UserConstructionScript`)