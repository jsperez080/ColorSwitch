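; Teleport puzzle controller that tracks the level's lever switches and shows their progress on a set of room lights.
; BeginPlay gathers every BP_LeverSwitch and builds the light array; each Tick lights the entry whose index matches an activated lever.
; Once all levers are active, it changes RoomLight9's material, plays a placeholder success sound and closes the Tick gate.
; Lever-to-light pairing depends on GetAllActorsOfClass order.
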(event `self.ReceiveBeginPlay`
  ;[1 1 1] Establish Initial Values
  (bind _outactors (`GameplayStatics.GetAllActorsOfClass` "/Game/GameContent/Obstacles/TeleportPuzzle/Switches/BP_LeverSwitch.BP_LeverSwitch_C"))
  (set `self.LeverSwitches` _outactors)
  (set `self.RoomLights` (`|MakeArray` (`self.RoomLight1`) (`self.RoomLight2`) (`self.RoomLight3`) (`self.RoomLight4`) (`self.RoomLight5`) (`self.RoomLight6`) (`self.RoomLight7`) (`self.RoomLight8`) (`self.RoomLight9`))))

(event `self.ReceiveTick`
  (params (DeltaSeconds :type "Float (single-precision)"))
  ;[1 1 1] Handle Puzzle Logic
  (`/Engine/EditorBlueprintResources/StandardMacros.Gate` false :!label _label
    (:`Exit`
      (`self.ActivateLightsOnPlatform`)
      (`self.ActivatePuzzleComplete`)
      (if (`self.AreAllRoomsActive`)
        (`/Engine/EditorBlueprintResources/StandardMacros.DoOnce` false
          (:`Completed`
            (`PrimitiveComponent.SetMaterial` (`self.RoomLight9`) 0 "/Game/GameContent/Obstacles/TeleportPuzzle/Materials/MI_AllRoomsActiveLight.MI_AllRoomsActiveLight")
            (`GameplayStatics.PlaySound2D` "/Game/GameContent/Obstacles/TeleportPuzzle/PlaceHolderSuccess.PlaceHolderSuccess" 1.0 1.0 0.0 null null)
            (goto _label :!via `Close`)))))))

(fn `ActivateLightsOnPlatform`
  (for (_array_element _array_index) (`self.LeverSwitches`)
    (set `self.LeverSwitchIndex` _array_index)
    (set `self.CurrentLeverSwitch` _array_element)
    (for (_ _array_index_2) (`self.RoomLights`)
      (set `self.RoomLightIndex` _array_index_2)
      (if (== (`self.LeverSwitchIndex`) (`self.RoomLightIndex`))
        (if (== (`/Game/GameContent/Obstacles/TeleportPuzzle/Switches/BP_LeverSwitch.IsActivated` (`self.CurrentLeverSwitch`)) true)
          (`PrimitiveComponent.SetMaterial` (`|GetArrayItem` (`self.RoomLights`) (`self.RoomLightIndex`)) 0 "/Game/GameContent/Obstacles/TeleportPuzzle/Materials/MI_RoomLightActive.MI_RoomLightActive"))))))

(fn `ActivatePuzzleComplete`
  (bind _alltrue (`self.AreAllActive`))
  (set `self.AreAllRoomsActive` _alltrue))

(fn `AreAllActive`
  (returns (AllTrue :type Boolean))
  (for _array_element (`self.LeverSwitches`)
    (if (not (`/Game/GameContent/Obstacles/TeleportPuzzle/Switches/BP_LeverSwitch.IsActivated` _array_element))
      (return false)))
  (return true))

(fn `UserConstructionScript`)