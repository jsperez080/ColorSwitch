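; BP_LeverSwitch is a lever for the teleport puzzle that the player pulls with the interact key.
; Overlapping its interaction volume as the player character enables input on the lever and shows a press-E widget.
; The interact action plays a timeline that rotates the lever on roll, then sets IsActivated when finished.
; Leaving the volume removes the widget but leaves input enabled, and nothing here resets the lever.
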(event `self.InteractCollision.OnComponentBeginOverlap`
  (params (OverlappedComponent :type "PrimitiveComponent Object Reference") (OtherActor :type "Actor Object Reference") (OtherComp :type "PrimitiveComponent Object Reference") (OtherBodyIndex :type Integer) (bFromSweep :type Boolean) (SweepResult :type "HitResult Structure (by ref)"))
  ;[1 1 1] On Overlap Allow player to interact with lever
  (cast `/Game/GameContent/PlayerCharacter/BP_PlayerCharacter` OtherActor)
  (`self.EnableInput` (`GameplayStatics.GetPlayerController` 0))
  (bind _returnvalue (`|CreateWidget` "/Game/GameContent/Obstacles/TeleportPuzzle/Switches/W_PressE.W_PressE_C"))
  (bind _output_get (set `self.PressEWidget` _returnvalue))
  (`UserWidget.AddToViewport` _output_get 0))

(event `InputAction|InteractionButton`
  (params (Key :type "Key Structure"))
  ;[1 1 1] Pull Lever upon player press [E], and set IsActive to true
  (:`Pressed`
    (bind (_direction _leverpull) (`Timeline|PullLever`)
      (:`Update`
        (`SceneComponent.K2_SetRelativeRotation` (`self.Lever`) (`KismetMathLibrary.MakeRotator` _leverpull) false false))
      (:`Finished`
        (set `self.IsActivated` true)))))

(event `self.InteractCollision.OnComponentEndOverlap`
  (params (OverlappedComponent :type "PrimitiveComponent Object Reference") (OtherActor :type "Actor Object Reference") (OtherComp :type "PrimitiveComponent Object Reference") (OtherBodyIndex :type Integer))
  ;[1 1 1] Remove interaction widget when player leaves collision volume
  (cast `/Game/GameContent/PlayerCharacter/BP_PlayerCharacter` OtherActor)
  (`Widget.RemoveFromParent` (`self.PressEWidget`)))

(fn `UserConstructionScript`)