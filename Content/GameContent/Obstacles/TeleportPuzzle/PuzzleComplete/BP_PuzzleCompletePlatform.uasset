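; Puzzle completion platform that unlocks once all teleport puzzle rooms are active, then descends when the player steps into its trigger box.
; Tick polls BP_TeleportLogic through a Gate, which closes after enabling movement and turning on the initially dark spotlight.
; A one-shot box overlap from BP_PlayerCharacter then plays a timeline that drives the platform's relative Z location.
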(event `self.ReceiveBeginPlay`
  ;[1 1 1] Set Initial Values and Set intensity of light to zero
  (bind _returnvalue (`GameplayStatics.GetActorOfClass` "/Game/GameContent/Obstacles/TeleportPuzzle/BP_TeleportLogic.BP_TeleportLogic_C"))
  (set `self.PuzzleLogicBP` _returnvalue)
  (`LightComponent.SetIntensity` (`self.SpotLight`) 0.0))

(event `self.ReceiveTick`
  (params (DeltaSeconds :type "Float (single-precision)"))
  ;[1 1 1] Check if All Rooms Active and Allow Player to overlap hitbox
  (`/Engine/EditorBlueprintResources/StandardMacros.Gate` false :!label _label
    (:`Exit`
      (if (`/Game/GameContent/Obstacles/TeleportPuzzle/BP_TeleportLogic.AreAllRoomsActive` (`self.PuzzleLogicBP`))
        (set `self.CanMove` true)
        (`LightComponent.SetIntensity` (`self.SpotLight`) 100000.0)
        (goto _label :!via `Close`)))))

(event `self.Box.OnComponentBeginOverlap`
  (params (OverlappedComponent :type "PrimitiveComponent Object Reference") (OtherActor :type "Actor Object Reference") (OtherComp :type "PrimitiveComponent Object Reference") (OtherBodyIndex :type Integer) (bFromSweep :type Boolean) (SweepResult :type "HitResult Structure (by ref)"))
  ;[1 1 1] Descend platform only when player has solved puzzle
  (cast `/Game/GameContent/PlayerCharacter/BP_PlayerCharacter` OtherActor)
  (if (`self.CanMove`)
    (`/Engine/EditorBlueprintResources/StandardMacros.DoOnce` false
      (:`Completed`
        (bind (_direction _descend) (`Timeline|DescendPlatform`)
          (:`Update`
            (`SceneComponent.K2_SetRelativeLocation` (`self.DescendingPlatform`) (`KismetMathLibrary.MakeVector` 0.0 0.0 _descend) false false)))))))

(fn `UserConstructionScript`)