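; Light/dark puzzle controller that lowers fences once all five child BP_ColorPuzzleParent pieces share the same value.
; Tick polls IsHit on four pieces and changes hardwired neighbours through ChangeAdjacent; Dark3 has no hit rule.
; GetPuzzleValues gathers one piece value per Tick, then compares the array against all-light and all-dark patterns.
; A match plays the MoveWallZ timeline, offsetting Fences down from the location cached in the construction script.
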(event `self.ReceiveBeginPlay`
  ;[1 1 1] Set Puzzle Pieces to Different Values
  (`self.SetPuzzlePieces`))

(event `self.ReceiveTick`
  (params (DeltaSeconds :type "Float (single-precision)"))
  (`|ExecutionSequence`
    (:`then_0`
      (`self.ChangeOne` (`self.Dark1`))
      (`self.ChangeOneAlt` (`self.Light2`)))
    (:`then_1`
      (`self.ChangeTwo` (`self.Dark2`)))
    (:`then_2`
      (`self.ChangeThree` (`self.Light1`)))
    (:`then_3`
      ;[1 1 1] Compare All values of puzzle and activate timeline if they are all identical
      (bind _allequal (`self.GetPuzzleValues`))
      (if _allequal
        (bind (_direction _movewallz) (`Timeline|MoveWallZ`)
          (:`Update`
            (`SceneComponent.K2_SetWorldLocation` (`self.Fences`) (`KismetMathLibrary.MakeVector` (.x (`self.InitialLocation`)) (.y (`self.InitialLocation`)) (- (.z (`self.InitialLocation`)) _movewallz)) false false)))))))

(fn `ChangeAdjacent`
  (params (Child1 :type "ChildActorComponent Object Reference"))
  (bind _asbp_color_puzzle_parent (cast `/Game/GameContent/Obstacles/Puzzle_01/BP_ColorPuzzleParent` (`ChildActorComponent.ChildActor` Child1)))
  (`/Game/GameContent/Obstacles/Puzzle_01/BP_ColorPuzzleParent.ChangeAdjacentPuzzlePiece` _asbp_color_puzzle_parent _asbp_color_puzzle_parent))

(fn `ChangeOne`
  (params (ChildPoint :type "ChildActorComponent Object Reference"))
  (bind _asbp_color_puzzle_parent (cast `/Game/GameContent/Obstacles/Puzzle_01/BP_ColorPuzzleParent` (`ChildActorComponent.ChildActor` ChildPoint)))
  (if (`/Game/GameContent/Obstacles/Puzzle_01/BP_ColorPuzzleParent.IsHit` _asbp_color_puzzle_parent)
    (`self.ChangeAdjacent` (`self.Light1`))
    (set `/Game/GameContent/Obstacles/Puzzle_01/BP_ColorPuzzleParent.IsHit` false _asbp_color_puzzle_parent)))

(fn `ChangeOneAlt`
  (params (Child :type "ChildActorComponent Object Reference"))
  (bind _asbp_color_puzzle_parent (cast `/Game/GameContent/Obstacles/Puzzle_01/BP_ColorPuzzleParent` (`ChildActorComponent.ChildActor` Child)))
  (if (`/Game/GameContent/Obstacles/Puzzle_01/BP_ColorPuzzleParent.IsHit` _asbp_color_puzzle_parent)
    (`self.ChangeAdjacent` (`self.Dark3`))
    (set `/Game/GameContent/Obstacles/Puzzle_01/BP_ColorPuzzleParent.IsHit` false _asbp_color_puzzle_parent)))

(fn `ChangeThree`
  (params (Child :type "ChildActorComponent Object Reference"))
  (bind _asbp_color_puzzle_parent (cast `/Game/GameContent/Obstacles/Puzzle_01/BP_ColorPuzzleParent` (`ChildActorComponent.ChildActor` Child)))
  (if (`/Game/GameContent/Obstacles/Puzzle_01/BP_ColorPuzzleParent.IsHit` _asbp_color_puzzle_parent)
    (`self.ChangeAdjacent` (`self.Dark2`))
    (`self.ChangeAdjacent` (`self.Dark3`))
    (`self.ChangeAdjacent` (`self.Light2`))
    (set `/Game/GameContent/Obstacles/Puzzle_01/BP_ColorPuzzleParent.IsHit` false _asbp_color_puzzle_parent)))

(fn `ChangeTwo`
  (params (Child :type "ChildActorComponent Object Reference"))
  (bind _asbp_color_puzzle_parent (cast `/Game/GameContent/Obstacles/Puzzle_01/BP_ColorPuzzleParent` (`ChildActorComponent.ChildActor` Child)))
  (if (`/Game/GameContent/Obstacles/Puzzle_01/BP_ColorPuzzleParent.IsHit` _asbp_color_puzzle_parent)
    (`self.ChangeAdjacent` (`self.Dark1`))
    (`self.ChangeAdjacent` (`self.Light2`))
    (set `/Game/GameContent/Obstacles/Puzzle_01/BP_ColorPuzzleParent.IsHit` false _asbp_color_puzzle_parent)))

(fn `GetPuzzleValues`
  (returns (AllEqual :type Boolean))
  (if (< (`self.iterator`) 5)
    (`KismetArrayLibrary.Array_Add` (`self.PiecesValue`) (`/Game/GameContent/Obstacles/Puzzle_01/BP_ColorPuzzleParent.LightDarkValue` (`|GetArrayItem` (`self.Pieces`) (`self.iterator`))))
    (`/Engine/EditorBlueprintResources/StandardMacros.IncrementInt` (`self.iterator`))
    (elif (or (`KismetArrayLibrary.Array_Identical` (`self.PiecesValue`) (`self.AllLight`)) (`KismetArrayLibrary.Array_Identical` (`self.PiecesValue`) (`self.AllDark`)))
      (set `self.AreAllSame` true)
      (return true)
      (else
        (set `self.iterator` 0)
        (`KismetArrayLibrary.Array_Clear` (`self.PiecesValue`))))))

(fn `SetPuzzlePieces`
  (`|ExecutionSequence`
    (:`then_0`
      (bind _asbp_color_puzzle_parent (cast `/Game/GameContent/Obstacles/Puzzle_01/BP_ColorPuzzleParent` (`ChildActorComponent.ChildActor` (`self.Dark1`)))))
    (:`then_1`
      (bind _asbp_color_puzzle_parent_2 (cast `/Game/GameContent/Obstacles/Puzzle_01/BP_ColorPuzzleParent` (`ChildActorComponent.ChildActor` (`self.Dark2`)))))
    (:`then_2`
      (bind _asbp_color_puzzle_parent_3 (cast `/Game/GameContent/Obstacles/Puzzle_01/BP_ColorPuzzleParent` (`ChildActorComponent.ChildActor` (`self.Dark3`)))))
    (:`then_3`
      (bind _asbp_color_puzzle_parent_4 (cast `/Game/GameContent/Obstacles/Puzzle_01/BP_ColorPuzzleParent` (`ChildActorComponent.ChildActor` (`self.Light1`)))))
    (:`then_4`
      (bind _asbp_color_puzzle_parent_5 (cast `/Game/GameContent/Obstacles/Puzzle_01/BP_ColorPuzzleParent` (`ChildActorComponent.ChildActor` (`self.Light2`)))))
    (:`then_5`
      (set `self.Pieces` (`|MakeArray` _asbp_color_puzzle_parent _asbp_color_puzzle_parent_2 _asbp_color_puzzle_parent_3 _asbp_color_puzzle_parent_4 _asbp_color_puzzle_parent_5)))))

(fn `UserConstructionScript`
  (set `self.InitialLocation` (`SceneComponent.K2_GetComponentLocation` (`self.Fences`))))