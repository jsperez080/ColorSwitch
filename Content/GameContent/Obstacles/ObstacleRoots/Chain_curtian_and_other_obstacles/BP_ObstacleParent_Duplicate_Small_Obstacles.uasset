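; Parent Blueprint for small light/dark obstacles that can move along a spline, spin, or be knocked out by projectiles.
; BeginPlay starts two chained timelines that ping-pong the mesh along the spline when CanMove is set; Tick applies yaw when CanRotate is set.
; Opposite-value projectile hits hide the mesh and disable its collision for five seconds when CanDisableObject is set.
; Tick compares the player's light/dark state, but both branches block Pawn.
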(event `self.ReceiveBeginPlay`
  (`self.SetCharacterTagValue`)
  (if (`self.CanMove`)
    (`self.MovePlatform`)
    (set `self.Initial Mesh Rotation` (`SceneComponent.K2_GetComponentRotation` (`self.Mesh`)))))

(event `self.Mesh.OnComponentHit`
  (params (HitComponent :type "PrimitiveComponent Object Reference") (OtherActor :type "Actor Object Reference") (OtherComp :type "PrimitiveComponent Object Reference") (NormalImpulse :type "Vector Structure") (Hit :type "HitResult Structure (by ref)"))
  ;[1 1 1] Toggle Collision and Visibility of Hit object
  (if (`self.CanDisableObject`)
    (bind _asbp_projectile_parent (cast `/Game/GameContent/Projectiles/Blueprints/BP_ProjectileParent` OtherActor))
    (if (`|EnumInequality` (`/Game/GameContent/Projectiles/Blueprints/BP_ProjectileParent.ProjectileValue` _asbp_projectile_parent) (`self.LightDarkValue`))
      (`SceneComponent.ToggleVisibility` (`self.Mesh`) false)
      (`PrimitiveComponent.SetCollisionEnabled` (`self.Mesh`) "NoCollision")
      (`KismetSystemLibrary.Delay` 5.0)
      (`SceneComponent.ToggleVisibility` (`self.Mesh`) false)
      (`PrimitiveComponent.SetCollisionEnabled` (`self.Mesh`) "QueryAndPhysics"))))

(event `MovePlatform`
  (bind _spline (`self.Spline`))
  (bind _spline_2 (`self.Spline`))
  ;[1 1 1] Loop Platform to move along Spline
  ;[1 1 1] Platform Movement that's not dependent on a time delay
  (bind (_direction _animationalpha) (`Timeline|Timeline_1` :!label _label)
    (:`Update`
      (bind _returnvalue (* _animationalpha (`SplineComponent.GetSplineLength` _spline_2)))
      (`SceneComponent.K2_SetWorldLocationAndRotation` (`self.Mesh`) (`SplineComponent.GetLocationAtDistanceAlongSpline` (`self.Spline`) _returnvalue "World") (`SplineComponent.GetRotationAtDistanceAlongSpline` _spline_2 _returnvalue "World") false false))
    (:`Finished`
      (bind (_direction_2 _animationalpha_2) (`Timeline|Timeline_2` :!via `ReverseFromEnd`)
        (:`Update`
          (bind _returnvalue_2 (* _animationalpha_2 (`SplineComponent.GetSplineLength` _spline)))
          (`SceneComponent.K2_SetWorldLocationAndRotation` (`self.Mesh`) (`SplineComponent.GetLocationAtDistanceAlongSpline` (`self.Spline`) _returnvalue_2 "World") (`SplineComponent.GetRotationAtDistanceAlongSpline` _spline _returnvalue_2 "World") false false))
        (:`Finished`
          (goto _label :!via `PlayFromStart`))))))

(event `self.ReceiveTick`
  (params (DeltaSeconds :type "Float (single-precision)"))
  ;[1 1 1] Only collide with player if they are the same color as this platform
  (if (`self.Can Rotate`)
    (`SceneComponent.K2_AddRelativeRotation` (`self.Mesh`) (`KismetMathLibrary.MakeRotator` 0.0 0.0 (* DeltaSeconds (`self.Rotation Multiplier`))) false false))
  (bind _outactors (`GameplayStatics.GetAllActorsOfClass` "/Game/GameContent/PlayerCharacter/BP_PlayerCharacter.BP_PlayerCharacter_C"))
  (if (`|EnumEquality` (`/Game/GameContent/PlayerCharacter/BP_PlayerCharacter.E Light Dark` (`|GetArrayItem` _outactors)) (`self.LightDarkValue`))
    (`PrimitiveComponent.SetCollisionResponseToChannel` (`self.Mesh`) "ECC_Pawn" "ECR_Block")
    (else
      (`PrimitiveComponent.SetCollisionResponseToChannel` (`self.Mesh`) "ECC_Pawn" "ECR_Block"))))

(fn `SetCharacterTagValue`)

(fn `UserConstructionScript`)